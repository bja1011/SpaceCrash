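; Asteroid field actor that scatters randomized instanced asteroids in a spherical shell, with every fiftieth spawn a fuel cube instead.
; Construction script fills the two instanced mesh components and records the fuel total.
; Tick rotates each asteroid by an index-scaled amount, with HardMode from the game instance swapping compose order so asteroids orbit the origin instead of spinning in place.
; Tick also pushes remaining and total fuel counts to the FlyingPawn.
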(event EventTick
  (params (DeltaSeconds :type Float%20%28single-precision%29))
  (bind _instancedstaticmesh (Variables|Default|GetInstancedStaticMesh))
  (for _index (range 0 (Components|InstancedStaticMesh|GetInstanceCount _instancedstaticmesh))
    (bind _returnvalue (CallFunction|HandleDiffcultyLevel (Math|Transform|MakeTransform "0, 0, 0" (Math|Rotator|MakeRotator (* _index 0.0001) (* _index 0.0001) (* _index 0.0001))) (.OutInstanceTransform (Components|InstancedStaticMesh|GetInstanceTransform _instancedstaticmesh _index false)) (Variables|Default|GetHardMode)))
    (Components|InstancedStaticMesh|UpdateInstanceTransform _instancedstaticmesh _index _returnvalue false true false)
    (bind _asflying_pawn (Utilities|Casting|CastToFlyingPawn (Game|Player|GetPlayerPawn 0)))
    (bind _output_get (Variables|/Game/FlyingBP/Blueprints/FlyingPawn.FlyingPawn_C|SetCubesLeft _asflying_pawn (Components|InstancedStaticMesh|GetInstanceCount (Variables|Default|GetFuel))))
    (Variables|/Game/FlyingBP/Blueprints/FlyingPawn.FlyingPawn_C|SetCubesTotal _asflying_pawn (Variables|Default|GetCubesTotal))
    (if (<= _output_get 79)
      _)))

(event Collision|EventActorBeginOverlap
  (params (OtherActor :type Actor%20Object%20Reference)))

(event EventBeginPlay
  (bind _asmy_game_instance (Utilities|Casting|CastToMyGameInstance (Game|GetGameInstance)))
  (Variables|Default|SetHardMode (Variables|/Game/MyGameInstance.MyGameInstance_C|GethardMode _asmy_game_instance)))

(fn ConstructionScript
  (bind _returnvalue (Math|Random|RandomUnitVector))
  (bind _returnvalue_2 (Math|Random|RandomRotator false))
  (bind _returnvalue_3 (Math|Random|RandomFloatinRange 0.0 2.0))
  (bind _mindistance (Variables|Default|GetMinDistance))
  (bind _maxdistance (Variables|Default|GetMaxDistance))
  (bind _returnvalue_4 (Math|Rotator|GetRotationXVector _returnvalue_2))
  (bind _returnvalue_5 (Math|Random|RandomFloatinRange _mindistance _maxdistance))
  (bind _returnvalue_6 (Math|Conversions|RotationFromXVector _returnvalue_4))
  (bind _returnvalue_7 (+ _returnvalue_3 _returnvalue_5))
  (bind _returnvalue_8 (* _returnvalue _returnvalue_7))
  (for _index (range 0 (Variables|Default|GetTotalCount))
    (switch int (Math|Integer|%(Integer) _index 50)
      (:Default
        (Components|InstancedStaticMesh|AddInstance (Variables|Default|GetInstancedStaticMesh) (Math|Transform|MakeTransform _returnvalue_8 _returnvalue_6 (Math|Conversions|ToVector(Float) (* (Math|Random|RandomFloatinRange (Variables|Default|GetMinScale) (Variables|Default|GetMaxScale)) (Variables|Default|GetScaleMultiplier))))))
      (:0
        (Components|InstancedStaticMesh|AddInstance (Variables|Default|GetFuel) (Math|Transform|MakeTransform _returnvalue_8 _returnvalue_6 "200.000000,200.000000,200.000000"))
        (Variables|Default|SetCubesTotal (Components|InstancedStaticMesh|GetInstanceCount (Variables|Default|GetFuel)))))))

(fn HandleDiffcultyLevel
  (params (InstanceTransform :type Transform%20%28by%20ref%29) (Transorm :type Transform%20%28by%20ref%29) (HardMode :type Boolean))
  (if HardMode
    (return (Math|Transform|ComposeTransforms Transorm InstanceTransform))
    (else
      (return (Math|Transform|ComposeTransforms InstanceTransform Transorm)))))