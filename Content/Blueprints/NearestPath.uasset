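; NearestPath actor that points from a source actor to the nearest instance in the Asteroids' Fuel instanced mesh with a thick pink debug line.
; When no target is set, Tick scans all instances by distance once and caches the result, then draws the line on subsequent frames.
; FindNearestBox clears the cache to trigger a new scan.
; The first instance only seeds the distance, so it never becomes TargetLocation.
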(event Custom|FindNearestBox
  (Variables|Default|SettargetLocation "0, 0, 0")
  (Variables|Default|SetlastDistance 0.0)
  (Variables|Default|SettargetSet false))

(event EventBeginPlay)

(event Collision|EventActorBeginOverlap
  (params (OtherActor :type Actor%20Object%20Reference)))

(event EventTick
  (params (DeltaSeconds :type Float%20%28single-precision%29))
  (bind _sourceactor (Variables|Default|GetsourceActor))
  (bind _asteroids (Variables|Default|Getasteroids))
  (bind _fuel (Variables|/Game/Environment/Blueprints/AsteroidsBP.AsteroidsBP_C|GetFuel _asteroids))
  (if (Variables|Default|GettargetSet)
    (Rendering|Debug|DrawDebugLine (+ (.location (Transformation|GetActorTransform _sourceactor)) (* (Transformation|GetActorForwardVector _sourceactor) 5e+01)) (Variables|Default|GettargetLocation) "(R=1.000000,G=0.045752,B=0.902677,A=1.000000)" 0.0 5e+01)
    (else
      (for _index (range 0 (Components|InstancedStaticMesh|GetInstanceCount _fuel))
        (if (== (Variables|Default|GetlastDistance) 0.0)
          (Variables|Default|SetlastDistance (Math|Vector|Distance(Vector) (.location (Transformation|GetActorTransform (Variables|Default|GetsourceActor))) (.location (.OutInstanceTransform (Components|InstancedStaticMesh|GetInstanceTransform _fuel _index true)))))
          (elif (< (Math|Vector|Distance(Vector) (.location (Transformation|GetActorTransform (Variables|Default|GetsourceActor))) (.location (.OutInstanceTransform (Components|InstancedStaticMesh|GetInstanceTransform _fuel _index true)))) (Variables|Default|GetlastDistance))
            (Variables|Default|SettargetLocation (.location (.OutInstanceTransform (Components|InstancedStaticMesh|GetInstanceTransform _fuel _index true))))
            (Variables|Default|SetlastDistance (Math|Vector|Distance(Vector) (.location (Transformation|GetActorTransform (Variables|Default|GetsourceActor))) (.location (.OutInstanceTransform (Components|InstancedStaticMesh|GetInstanceTransform _fuel _index true))))))))
      (Variables|Default|SettargetSet true))))

(fn ConstructionScript)